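; Enemy character that wanders, chases pawns it sees and attacks them in melee.
; Patrol loops AIMoveTo to random reachable points, while PawnSensing triggers a chase that falls back to patrol on failure.
; On arrival it plays an attack montage, then sphere-traces at its mesh and calls ApplyDamage with no amount set.
; TakeDamage negates Health rather than subtracting, then plays a hit montage or a death montage before destroying the actor.
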(event OnSeePawn(PawnSensing)
  (params (Pawn :type Pawn%20Object%20Reference))
  (CallFunction|ChaseTarget Pawn))

(event Custom|Take%20Damage
  (Variables|Default|SetHealth (- 0.0 (Variables|Default|GetHealth)))
  (if (<= (Variables|Default|GetHealth) 0.0)
    (bind _returnvalue (Animation|PlayAnimMontage "/Game/Animations/Enemie_Animations/AM_Death.AM_Death" 1.0 "None"))
    (Utilities|FlowControl|Delay _returnvalue)
    (Actor|DestroyActor)
    (else
      (Animation|PlayAnimMontage "/Game/Animations/Enemie_Animations/AM_Hit.AM_Hit" 1.0 "None"))))

(event Custom|Patrol
  (AI|AIMoveTo self (.RandomLocation (AI|Navigation|GetRandomReachablePointinRadius (Transformation|GetActorLocation) 1e+03 0 0)) 0 5.0 false
    (:OnSuccess
      (Utilities|FlowControl|Delay 1.0))
    (:OnFail
      _))
  (CallFunction|Patrol))

(event Custom|Chase%20Target
  (params (TargetActor :type Actor%20Object%20Reference))
  (bind _mesh (Variables|Character|GetMesh))
  (bind _returnvalue (Transformation|GetWorldLocation _mesh))
  (if (Variables|Default|GetcanMove?)
    (AI|AIMoveTo self "0, 0, 0" TargetActor 2e+01 false
      (:OnSuccess
        (Variables|Default|SetcanMove? false)
        (if (Variables|Default|GetcanAttack?)
          (Animation|PlayAnimMontage "/Game/Animations/Enemie_Animations/AM_Attack.AM_Attack" 1.0 "None")
          (Utilities|FlowControl|Delay 1.0)
          (Variables|Default|SetcanAttack? false)
          (bind (_outhit _returnvalue_2) (Collision|SphereTraceForObjects _returnvalue _returnvalue 1e+02 (Utilities|Array|MakeArray "ObjectTypeQuery3") false 0 "ForDuration" true "(R=1.000000,G=0.000000,B=0.000000,A=1.000000)" "(R=0.000000,G=1.000000,B=0.000000,A=1.000000)" 1.0))
          (if _returnvalue_2
            (Development|PrintString "Recibiste daño")
            (Game|Damage|ApplyDamage (.HitActor (Collision|BreakHitResult _outhit)) 0.0 0 0)
            (else
              (Development|PrintString "No Pego")))
          (Variables|Default|SetcanAttack? true)
          (Variables|Default|SetcanMove? true)
          (Variables|Default|SetIsSeeingPlayer? true)))
      (:OnFail
        (CallFunction|Patrol)
        (Variables|Default|SetcanMove? true)))))

(event EventBeginPlay
  (CallFunction|Patrol))

(fn ConstructionScript)