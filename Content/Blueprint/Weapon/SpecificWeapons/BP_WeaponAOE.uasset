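; BP_WeaponAOE is a weapon Blueprint that attacks by spawning an area-of-effect bullet, BP_AOEBullet.
; FnAttack checks IsReadyToAttack, calls Attacked, then spawns the bullet at the given start point and rotation with the instigator as its ActorOwner.
; A Delay of AttackCooldown ends the chain with nothing wired after it, so this graph does not itself reset readiness.
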(event EventBeginPlay
  (|CallParentFunction) ; This node is disabled and will not be called.\nDrag off pins to build functionality.
)

(event Collision|EventActorBeginOverlap
  (params (OtherActor :type Actor%20Object%20Reference))
  (|CallParentFunction OtherActor) ; This node is disabled and will not be called.\nDrag off pins to build functionality.
)

(event EventTick
  (params (DeltaSeconds :type Float%20%28single-precision%29))
  (|CallParentFunction DeltaSeconds) ; This node is disabled and will not be called.\nDrag off pins to build functionality.
)

(event EventFnAttack
  (params (Instigator :type Actor%20Object%20Reference) (StartPoint :type Vector :default "0, 0, 0") (Rotation :type Rotator :default "0, 0, 0"))
  (if (Variables|Default|GetIsReadyToAttack)
    (CallFunction|Attacked)
    (bind _returnvalue (Game|SpawnActorfromClass "/Game/Blueprint/Projectiles/BP_AOEBullet.BP_AOEBullet_C" (Math|Transform|MakeTransform StartPoint Rotation "1.000000,1.000000,1.000000") "Undefined" "MultiplyWithRoot" 0 0))
    (Variables|/Game/Blueprint/Projectiles/BP_Bullet.BP_Bullet_C|SetActorOwner _returnvalue Instigator)
    (Utilities|FlowControl|Delay (Variables|Default|GetAttackCooldown))))

(fn ConstructionScript
  (|CallParentFunction))