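; BP_WeaponMele is a melee weapon Blueprint that deals area damage around a given start point when it attacks.
; FnAttack checks IsReadyToAttack, calls Attacked, then runs a zero-length multi sphere trace on the Visibility channel with debug drawing.
; Hit actors implementing BPI_Damagable receive FnDamage with the weapon's owner as causer and DamageAmount as the damage.
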(event EventBeginPlay
  (|CallParentFunction) ; This node is disabled and will not be called.\nDrag off pins to build functionality.
)

(event Collision|EventActorBeginOverlap
  (params (OtherActor :type Actor%20Object%20Reference))
  (|CallParentFunction OtherActor) ; This node is disabled and will not be called.\nDrag off pins to build functionality.
)

(event EventTick
  (params (DeltaSeconds :type Float%20%28single-precision%29))
  (|CallParentFunction DeltaSeconds) ; This node is disabled and will not be called.\nDrag off pins to build functionality.
)

(event EventFnAttack
  (params (Instigator :type Actor%20Object%20Reference) (StartPoint :type Vector :default "0, 0, 0") (Rotation :type Rotator :default "0, 0, 0"))
  (if (Variables|Default|GetIsReadyToAttack)
    (CallFunction|Attacked)
    (bind (_outhits _returnvalue) (Collision|MultiSphereTraceByChannel StartPoint StartPoint (Variables|Default|GetAttackRadius) "TraceTypeQuery1" false 0 "ForDuration" true "(R=1.000000,G=0.000000,B=0.000000,A=1.000000)" "(R=0.000000,G=1.000000,B=0.000000,A=1.000000)" 2.0))
    (if _returnvalue
      (for _array_element _outhits
        (bind _asbpi_damagable (Utilities|Casting|CastToBPI_Damagable (.HitActor (Collision|BreakHitResult _array_element))))
        (Default|FnDamage _asbpi_damagable (Components|GetOwner) (Variables|Default|GetDamageAmount))))))

(fn ConstructionScript
  (|CallParentFunction))