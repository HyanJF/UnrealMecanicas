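; Area-of-effect projectile that deals explosion damage around itself when it is destroyed.
; On Destroyed, it runs a stationary multi sphere trace on the Visibility channel at the mesh location, using AOERange as the radius.
; Each hit actor other than the owner that implements BPI_Damagable receives ExplotionDamage through FnDamage, with the owner as causer.
; Debug print and trace drawing are left on.
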(event EventBeginPlay
  (|CallParentFunction) ; This node is disabled and will not be called.\nDrag off pins to build functionality.
)

(event Collision|EventActorBeginOverlap
  (params (OtherActor :type Actor%20Object%20Reference))
  (|CallParentFunction OtherActor) ; This node is disabled and will not be called.\nDrag off pins to build functionality.
)

(event EventTick
  (params (DeltaSeconds :type Float%20%28single-precision%29))
  (|CallParentFunction DeltaSeconds) ; This node is disabled and will not be called.\nDrag off pins to build functionality.
)

(event EventDestroyed
  (bind _mesh (Variables|Character|GetMesh))
  (bind _returnvalue (Transformation|GetWorldLocation _mesh))
  (Development|PrintString "AOE" true true "(R=0.000000,G=0.660000,B=1.000000,A=1.000000)" 2.0 "Destroyed")
  (bind (_outhits _returnvalue_2) (Collision|MultiSphereTraceByChannel _returnvalue _returnvalue (Variables|Default|GetAOERange) "TraceTypeQuery1" false 0 "ForDuration" true "(R=1.000000,G=0.000000,B=0.000000,A=1.000000)" "(R=0.000000,G=1.000000,B=0.000000,A=1.000000)" 2.0))
  (if _returnvalue_2
    (bind _array_element (Utilities|Array|ForEachLoopwithBreak _outhits)
      (:LoopBody
        (if (!= (.HitActor (Collision|BreakHitResult _array_element)) (Variables|Default|GetActorOwner))
          (bind _asbpi_damagable (Utilities|Casting|CastToBPI_Damagable (.HitActor (Collision|BreakHitResult _array_element))))
          (Default|FnDamage _asbpi_damagable (Variables|Default|GetActorOwner) (Variables|Default|GetExplotionDamage)))))))

(fn ConstructionScript
  (|CallParentFunction))