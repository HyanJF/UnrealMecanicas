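; Projectile bullet actor that flies forward, damages what it hits and destroys itself when its lifetime runs out.
; Tick moves the root along local X at Speed with an unswept offset, without using a projectile movement component.
; With a valid ActorOwner, overlapping any other actor applies damage through BPI_Damagable where implemented, crediting the owner, then destroys the bullet.
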(event OnComponentBeginOverlap(Collision)
  (params (OverlappedComponent :type Primitive%20Component%20Object%20Reference) (OtherActor :type Actor%20Object%20Reference) (OtherComp :type Primitive%20Component%20Object%20Reference) (OtherBodyIndex :type Integer) (bFromSweep :type Boolean) (SweepResult :type Hit%20Result%20Structure%20%28by%20ref%29))
  (Utilities|IsValid (Variables|Default|GetActorOwner)
    (:Is%20Valid
      (if (!= OtherActor (Variables|Default|GetActorOwner))
        (bind _asbpi_damagable (Utilities|Casting|CastToBPI_Damagable OtherActor)
          (:then
            (Default|FnDamage _asbpi_damagable (Variables|Default|GetActorOwner) (Variables|Default|GetDamage)))
          (:CastFailed
            _))
        (Actor|DestroyActor)))))

(event EventBeginPlay
  (Utilities|FlowControl|Delay (Variables|Default|GetLifetime))
  (Actor|DestroyActor))

(event EventTick
  (params (DeltaSeconds :type Float%20%28single-precision%29))
  (Transformation|AddLocalOffset (Variables|Default|GetDefaultSceneRoot) (Math|Vector|MakeVector (* DeltaSeconds (Variables|Default|GetSpeed)) 0.0 0.0) false false))

(fn ConstructionScript)