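; Player component for a build mode that places new chairs or moves existing ones.
; While active, a per-tick camera line trace positions a rotatable chair preview, with DoOnce-gated material swaps showing whether the hit actor is tagged Buildable.
; On valid placement it spawns BP_BuildChair or repositions the hidden original, then requests a save through the game instance.
; Leaving build mode clears the preview and restores any moved build's visibility and collision.
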(event Custom|Preview%20Loop
  (bind _camera (Variables|Default|GetCamera))
  (bind _returnvalue (Transformation|GetWorldTransform _camera))
  ;[0.15 0.15 0.15 0.5] Build loop
  (bind (_outhit _returnvalue_2) (Collision|LineTraceByChannel (.location _returnvalue) (+ (.location _returnvalue) (* (Math|Vector|GetForwardVector (.rotation _returnvalue)) (Variables|Default|GetRayDistance))) "TraceTypeQuery1" false 0 "ForOneFrame"))
  (if _returnvalue_2
    (Utilities|FlowControl|Sequence
      (:then_0
        (Utilities|FlowControl|DoOnce false
          (:Completed
            (CallFunction|SetPreviewMesh))))
      (:then_1
        (CallFunction|SetPreviewMeshPosition (.Location (Collision|BreakHitResult _outhit))))
      (:then_2
        (if (Actor|ActorHasTag (.HitActor (Collision|BreakHitResult _outhit)) "Buildable")
          (Utilities|FlowControl|DoOnce false
            (:Completed
              (Rendering|Material|SetMaterial (Variables|Default|GetPreview%20Mesh) 0 "/Game/Materials/PreviewMesh.PreviewMesh")
              (Variables|Default|SetCanBuild true)
              (CallFunction|ResetCantBuildMaterial)))
          (else
            (Utilities|FlowControl|DoOnce false
              (:Completed
                (Rendering|Material|SetMaterial (Variables|Default|GetPreview%20Mesh) 0 "/Game/Materials/MI_CantBuildPreviewMaterial.MI_CantBuildPreviewMaterial")
                (Variables|Default|SetCanBuild false)
                (CallFunction|ResetCanBuildMaterial)))))))))

(event Custom|ResetBuildMode
  ;[0.15 0.15 0.15 0.5] Build loop
  (Utilities|FlowControl|DoOnce false) ; enters at Reset
)

(event Custom|Stop%20Build%20Mode
  (bind _buildtomove (Variables|Default|GetBuildToMove))
  ;[0.15 0.15 0.15 0.5] Toggle build mode
  (Variables|Default|SetInBuildMode false)
  (Components|StaticMesh|SetStaticMesh (Variables|Default|GetPreview%20Mesh) 0)
  (Variables|Default|SetPreview%20Mesh 0)
  (CallFunction|ResetBuildMode)
  (Variables|Default|SetIsMovingBuild false)
  (Utilities|IsValid _buildtomove
    (:Is%20Valid
      (Collision|SetActorEnableCollision _buildtomove true)
      (Rendering|SetActorHiddenInGame _buildtomove false))))

(event Custom|SetBuildToMove
  (params (BuildToMove :type BP%20Buildable%20Object%20Object%20Reference))
  ;[0.15 0.15 0.15 0.5] Set build to move
  (Variables|Default|SetBuildToMove BuildToMove)
  (Collision|SetActorEnableCollision (Variables|Default|GetBuildToMove) false)
  (Rendering|SetActorHiddenInGame (Variables|Default|GetBuildToMove) true)
  (Variables|Default|SetIsMovingBuild true)
  (CallFunction|StartBuildingMode))

(event Custom|StartBuildingMode
  ;[0.15 0.15 0.15 0.5] Toggle build mode
  (Variables|Default|SetInBuildMode true)
  (CallFunction|ResetCanBuildMaterial)
  (CallFunction|ResetCantBuildMaterial))

(event Custom|ResetCantBuildMaterial
  ;[0.15 0.15 0.15 0.5] Build loop
  (Utilities|FlowControl|DoOnce false) ; enters at Reset
)

(event Custom|ResetCanBuildMaterial
  ;[0.15 0.15 0.15 0.5] Build loop
  (Utilities|FlowControl|DoOnce false) ; enters at Reset
)

(event Input|EnhancedActionEvents|EnhancedInputActionIA_Build
  (params (ActionValue :type Boolean) (ElapsedSeconds :type Float%20%28double-precision%29) (TriggeredSeconds :type Float%20%28double-precision%29) (InputAction :type Input%20Action%20Object%20Reference :default "/Game/FirstPerson/Input/Actions/IA_Build.IA_Build"))
  (bind _buildtomove (Variables|Default|GetBuildToMove))
  ;[0.15 0.15 0.15 0.5] Toggle build mode
  (:Started
    (if (Variables|Default|GetInBuildMode)
      (Variables|Default|SetInBuildMode false)
      (Components|StaticMesh|SetStaticMesh (Variables|Default|GetPreview%20Mesh) 0)
      (Variables|Default|SetPreview%20Mesh 0)
      (CallFunction|ResetBuildMode)
      (Variables|Default|SetIsMovingBuild false)
      (Utilities|IsValid _buildtomove
        (:Is%20Valid
          (Collision|SetActorEnableCollision _buildtomove true)
          (Rendering|SetActorHiddenInGame _buildtomove false)))
      (else
        (Variables|Default|SetInBuildMode true)
        (CallFunction|ResetCanBuildMaterial)
        (CallFunction|ResetCantBuildMaterial)))))

(event Input|EnhancedActionEvents|EnhancedInputActionIA_PlaceBuild
  (params (ActionValue :type Boolean) (ElapsedSeconds :type Float%20%28double-precision%29) (TriggeredSeconds :type Float%20%28double-precision%29) (InputAction :type Input%20Action%20Object%20Reference :default "/Game/FirstPerson/Input/Actions/IA_PlaceBuild.IA_PlaceBuild"))
  ;[0.15 0.15 0.15 0.5] Place build
  (:Started
    (if (and (Variables|Default|GetInBuildMode) (Variables|Default|GetCanBuild))
      (if (Variables|Default|GetIsMovingBuild)
        (Transformation|SetWorldTransform (Variables|/Game/Blueprint/Objects/Buildable/BP_BuildableObject.BP_BuildableObject_C|GetDefaultSceneRoot (Variables|Default|GetBuildToMove)) (Variables|Default|GetBuild%20Preview%20transform) false false)
        (Class|BPISaveGame|SaveChairs(Message) (Game|GetGameInstance) true)
        (else
          (Game|SpawnActorfromClass "/Game/Blueprint/Objects/Buildable/BP_BuildChair.BP_BuildChair_C" (Variables|Default|GetBuild%20Preview%20transform) "AdjustIfPossibleButAlwaysSpawn" "MultiplyWithRoot" 0 0)
          (Class|BPISaveGame|SaveChairs(Message) (Game|GetGameInstance) true)))
      (CallFunction|StopBuildMode))))

(event Input|EnhancedActionEvents|EnhancedInputActionIA_RotateBuild
  (params (ActionValue :type Float%20%28double-precision%29) (ElapsedSeconds :type Float%20%28double-precision%29) (TriggeredSeconds :type Float%20%28double-precision%29) (InputAction :type Input%20Action%20Object%20Reference :default "/Game/FirstPerson/Input/Actions/IA_RotateBuild.IA_RotateBuild"))
  ;[0.15 0.15 0.15 0.5] RotateBuilding
  (Variables|Default|SetBuildPreviewRotation (Math|Rotator|MakeRotator 0.0 0.0 (+ (* ActionValue (Variables|Default|GetRotation)) (.Yaw (Math|Rotator|BreakRotator (Variables|Default|GetBuildPreviewRotation)))))))

(event EventBeginPlay
  ;[0.15 0.15 0.15 0.5] BeginPlay
  (bind _asbp_first_person_player (Utilities|Casting|CastToBP_FirstPersonPlayer (Components|GetOwner)))
  (bind _output_get (Variables|Default|SetPlayer%20BP _asbp_first_person_player))
  (Variables|Default|SetCamera (Variables|/Game/Blueprint/Player/BP_FirstPersonPlayer.BP_FirstPersonPlayer_C|GetFirstPersonCamera _output_get)))

(event EventTick
  (params (DeltaSeconds :type Float%20%28single-precision%29))
  ;[0.15 0.15 0.15 0.5] Tick
  (if (Variables|Default|GetInBuildMode)
    (CallFunction|PreviewLoop)))

(fn SetPreviewMesh
  (bind _returnvalue (Game|AddComponentbyClass (Variables|Default|GetPlayer%20BP) "/Script/Engine.StaticMeshComponent" false (Variables|Default|GetBuild%20Preview%20transform)))
  (bind _output_get (Variables|Default|SetPreview%20Mesh _returnvalue))
  (Components|StaticMesh|SetStaticMesh _output_get "/Game/StarterContent/Props/SM_Chair.SM_Chair")
  (Collision|SetCollisionEnabled (Variables|Default|GetPreview%20Mesh) "NoCollision"))

(fn SetPreviewMeshPosition
  (params (Build%20Preview%20Location :type Vector))
  (bind _output_get (Variables|Default|SetBuild%20Preview%20transform (Math|Transform|MakeTransform Build%20Preview%20Location (Variables|Default|GetBuildPreviewRotation) "1.000000,1.000000,1.000000")))
  (Transformation|SetWorldTransform (Variables|Default|GetPreview%20Mesh) _output_get false false))