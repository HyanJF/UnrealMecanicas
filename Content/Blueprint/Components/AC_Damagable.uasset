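; AC_Damagable is an actor component that gives its owner hit points and a death notification.
; On BeginPlay it sets current HP to max HP and prints the value.
; Its FnDamage event ignores damage caused by the owner, subtracts the absolute amount otherwise, and calls the Die dispatcher once HP drops below zero.
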(event EventBeginPlay
  (bind _output_get (Variables|Default|SetCurrentHp (Variables|Default|GetMaxHp)))
  (Development|PrintString (Utilities|String|ToString(Float) _output_get)))

(event EventTick
  (params (DeltaSeconds :type Float%20%28single-precision%29)))

(event EventFnDamage
  (params (DamageCauser :type Actor%20Object%20Reference) (DamageAmount :type Float%20%28double-precision%29))
  (if (!= DamageCauser (Components|GetOwner))
    (bind _output_get (Variables|Default|SetCurrentHp (- (Variables|Default|GetCurrentHp) (Math|Float|Absolute(Float) DamageAmount))))
    (if (< _output_get 0.0)
      (Default|CallDie))))