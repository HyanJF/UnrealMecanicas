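; AC_WeaponHolder is a component that holds an array of weapons, handles switching between them and fires the active one.
; Attack forwards the start point and rotation to the current weapon's FnAttack, passing the component's owner as instigator.
; NextWeapon and PreviousWeapon hide the current weapon, step the index with modulo wraparound in both directions, then unhide the newly selected one.
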(event Custom|Attack
  (params (StartPoint :type Vector) (Rotation :type Rotator))
  (Default|FnAttack (Utilities|Array|Get(acopy) (Variables|Default|GetWeapons) (Variables|Default|GetCurrentWeapon)) (Components|GetOwner) StartPoint Rotation))

(event Custom|NextWeapon
  (bind _weapons (Variables|Default|GetWeapons))
  (bind _returnvalue (Utilities|Array|Length _weapons))
  (Rendering|SetActorHiddenInGame (Utilities|Array|Get(acopy) (Variables|Default|GetWeapons) (Variables|Default|GetCurrentWeapon)) true)
  (Math|Integer|IncrementInt (Variables|Default|GetCurrentWeapon)
    (:%20%20
      (bind _output_get (Variables|Default|SetCurrentWeapon (Math|Integer|%(Integer) (+ (Variables|Default|GetCurrentWeapon) _returnvalue) _returnvalue)))
      (Rendering|SetActorHiddenInGame (Utilities|Array|Get(acopy) (Variables|Default|GetWeapons) _output_get) false))))

(event Custom|PreviousWeapon
  (bind _weapons (Variables|Default|GetWeapons))
  (bind _returnvalue (Utilities|Array|Length _weapons))
  (Rendering|SetActorHiddenInGame (Utilities|Array|Get(acopy) (Variables|Default|GetWeapons) (Variables|Default|GetCurrentWeapon)) true)
  (Math|Integer|DecrementInt (Variables|Default|GetCurrentWeapon)
    (:%20%20
      (bind _output_get (Variables|Default|SetCurrentWeapon (Math|Integer|%(Integer) (+ (Variables|Default|GetCurrentWeapon) _returnvalue) _returnvalue)))
      (Rendering|SetActorHiddenInGame (Utilities|Array|Get(acopy) (Variables|Default|GetWeapons) _output_get) false))))

(event EventBeginPlay)

(event EventTick
  (params (DeltaSeconds :type Float%20%28single-precision%29)))