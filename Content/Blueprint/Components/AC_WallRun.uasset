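; AC_WallRun is a component that switches its owning character's movement into and out of a wall-run state.
; On BeginPlay it caches the owner's CharacterMovementComponent.
; EnterWallRun zeroes gravity scale and vertical velocity while keeping horizontal momentum, and ExitWallRun sets gravity scale back to a fixed default.
; It contains no wall detection or per-tick logic, only these two state-change events.
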(event EventBeginPlay
  (Variables|Default|SetCharachterMoveRef (Actor|GetComponentbyClass (Components|GetOwner) "/Script/Engine.CharacterMovementComponent")))

(event EventExitWallRun
  (Variables|/Script/Engine.CharacterMovementComponent|SetGravityScale (Variables|Default|GetCharachterMoveRef) 1.0))

(event EventEnterWallRun
  (bind _charachtermoveref (Variables|Default|GetCharachterMoveRef))
  (Variables|/Script/Engine.CharacterMovementComponent|SetGravityScale _charachtermoveref 0.0)
  (Variables|/Script/Engine.MovementComponent|SetVelocity _charachtermoveref (Math|Vector|MakeVector (.x (Variables|/Script/Engine.MovementComponent|GetVelocity _charachtermoveref)) (.y (Variables|/Script/Engine.MovementComponent|GetVelocity _charachtermoveref)) 0.0)))