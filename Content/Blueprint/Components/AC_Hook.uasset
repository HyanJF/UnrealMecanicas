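; Actor component that gives its owner a two-hook tool, pulling two hookable objects toward each other.
; At BeginPlay it spawns hidden purple and yellow hook actors; fire and alt-fire each place one via a camera line trace.
; A hit on an actor with AC_Hookable attaches the hook and stores that component.
; Once both points are set, each moves to the other and the hooks hide after a second.
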(event EventBeginPlay
  (Variables|Default|SetCamera (Actor|GetComponentbyClass (Components|GetOwner) "/Script/Engine.CameraComponent"))
  (bind _returnvalue (Game|SpawnActorfromClass "/Game/Blueprint/Objects/Hook/BP_Hook_Purple.BP_Hook_Purple_C" (Math|Transform|MakeTransform "0, 0, 0" "0, 0, 0" "1.000000,1.000000,1.000000") "Undefined" "MultiplyWithRoot" 0 0))
  (bind _output_get (Variables|Default|SetPurpleHook _returnvalue))
  (Rendering|SetActorHiddenInGame _output_get true)
  (bind _returnvalue_2 (Game|SpawnActorfromClass "/Game/Blueprint/Objects/Hook/BP_Hook_Yellow.BP_Hook_Yellow_C" (Math|Transform|MakeTransform "0, 0, 0" "0, 0, 0" "1.000000,1.000000,1.000000") "Undefined" "MultiplyWithRoot" 0 0))
  (bind _output_get_2 (Variables|Default|SetYellowHook _returnvalue_2))
  (Rendering|SetActorHiddenInGame _returnvalue_2 true))

(event EventFnAltFire
  (bind _hookedactor (CallFunction|MoveHook (Variables|Default|GetYellowHook)))
  (Utilities|IsValid _hookedactor
    (:Is%20Valid
      (Variables|Default|SetSecondPoint _hookedactor)
      (if (and (Utilities|IsValid (Variables|Default|GetFirstPoint)) (Utilities|IsValid (Variables|Default|GetSecondPoint)))
        (Default|FnMovetoTarge (Variables|Default|GetFirstPoint) (Variables|Default|GetSecondPoint))
        (Default|FnMovetoTarge (Variables|Default|GetSecondPoint) (Variables|Default|GetFirstPoint))
        (Variables|Default|SetFirstPoint 0)
        (Variables|Default|SetSecondPoint 0)
        (Utilities|FlowControl|Delay 1.0)
        (Rendering|SetActorHiddenInGame (Variables|Default|GetYellowHook) true)
        (Rendering|SetActorHiddenInGame (Variables|Default|GetPurpleHook) true)))))

(event EventFnFire
  (bind _hookedactor (CallFunction|MoveHook (Variables|Default|GetPurpleHook)))
  (Utilities|IsValid _hookedactor
    (:Is%20Valid
      (Variables|Default|SetFirstPoint _hookedactor)
      (if (and (Utilities|IsValid (Variables|Default|GetFirstPoint)) (Utilities|IsValid (Variables|Default|GetSecondPoint)))
        (Default|FnMovetoTarge (Variables|Default|GetFirstPoint) (Variables|Default|GetSecondPoint))
        (Default|FnMovetoTarge (Variables|Default|GetSecondPoint) (Variables|Default|GetFirstPoint))
        (Variables|Default|SetFirstPoint 0)
        (Variables|Default|SetSecondPoint 0)
        (Utilities|FlowControl|Delay 1.0)
        (Rendering|SetActorHiddenInGame (Variables|Default|GetYellowHook) true)
        (Rendering|SetActorHiddenInGame (Variables|Default|GetPurpleHook) true)))))

(fn MoveHook
  (params (Hook :type BP%20Hook%20Object%20Reference))
  (bind _camera (Variables|Default|GetCamera))
  (bind _returnvalue (Transformation|GetWorldLocation _camera))
  (bind (_outhit _returnvalue_2) (Collision|LineTraceByChannel _returnvalue (+ _returnvalue (* (Math|Vector|GetForwardVector _camera) (Variables|Default|GetRayDistance))) "TraceTypeQuery1" false 0 "None"))
  (if _returnvalue_2
    (Utilities|IsValid (Actor|GetComponentbyClass (.HitActor (Collision|BreakHitResult _outhit)) "/Game/Blueprint/Components/AC_Hookable.AC_Hookable_C")
      (:Is%20Valid
        (Rendering|SetActorHiddenInGame Hook true)
        (Transformation|SetActorTransform Hook (Math|Transform|MakeTransform (.Location (Collision|BreakHitResult _outhit)) (Math|Rotator|MakeRotfromZ (.Normal (Collision|BreakHitResult _outhit))) "1.000000,1.000000,1.000000") false true)
        (Default|FNAttachHook (Actor|GetComponentbyClass (.HitActor (Collision|BreakHitResult _outhit)) "/Game/Blueprint/Components/AC_Hookable.AC_Hookable_C") Hook)
        (Rendering|SetActorHiddenInGame Hook false)
        (return (Actor|GetComponentbyClass (.HitActor (Collision|BreakHitResult _outhit)) "/Game/Blueprint/Components/AC_Hookable.AC_Hookable_C")))
      (:Is%20Not%20Valid
        _)))
  (Transformation|DetachFromActor Hook "KeepRelative" "KeepRelative" "KeepRelative")
  (Rendering|SetActorHiddenInGame Hook true))