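; AC_Money is a component that holds a money balance with passive income over time.
; From BeginPlay, a looping one-second Retriggerable Delay feeds GainsPerSecond into the AddMoney event, which increases CurrentMoney.
; AskForMoney handles spending: it deducts the requested amount and returns true if the balance covers it, otherwise it returns false and leaves the balance unchanged.
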(event Custom|AddMoney
  (params (Amount :type Integer64))
  (Variables|Default|SetCurrentMoney (+ (Variables|Default|GetCurrentMoney) Amount)))

(event EventBeginPlay
  (Utilities|FlowControl|RetriggerableDelay 1.0 :!label _label)
  (CallFunction|AddMoney (Variables|Default|GetGainsPerSecond))
  (goto _label))

(fn AskforMoney
  (params (Amount :type Integer64))
  (if (<= Amount (Variables|Default|GetCurrentMoney))
    (Variables|Default|SetCurrentMoney (- (Variables|Default|GetCurrentMoney) Amount))
    (return true)
    (else
      (return false))))