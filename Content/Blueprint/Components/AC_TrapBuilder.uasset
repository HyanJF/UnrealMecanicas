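; Trap-building component for BP_OrcPlayer that lets the player place new builds or relocate existing ones.
; In build mode, a per-tick camera line trace moves a preview mesh to the hit point, aligned to the surface normal.
; The hit actor's "Buildable" tag drives preview visibility and CanBuild, with paired DoOnce nodes limiting material swaps to state changes.
; Placing spawns the selected build's class or teleports the hidden actor being moved, then exits build mode.
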(event Custom|Preview%20Loop
  (bind _camera (Variables|Default|GetCamera))
  (bind _returnvalue (Transformation|GetWorldTransform _camera))
  ;[0.15 0.15 0.15 0.5] Build loop
  (bind (_outhit _returnvalue_2) (Collision|LineTraceByChannel (.location _returnvalue) (+ (.location _returnvalue) (* (Math|Vector|GetForwardVector (.rotation _returnvalue)) (Variables|Default|GetRayDistance))) "TraceTypeQuery1" false 0 "ForOneFrame"))
  (if _returnvalue_2
    (Development|SetHiddeninGame (Variables|Default|GetPreview%20Mesh) (not (Actor|ActorHasTag (.HitActor (Collision|BreakHitResult _outhit)) "Buildable")) false)
    (CallFunction|SetAbletoBuild (Actor|ActorHasTag (.HitActor (Collision|BreakHitResult _outhit)) "Buildable"))
    (bind _output_get (Variables|Default|SetBuild%20Preview%20transform (Math|Transform|MakeTransform (.Location (Collision|BreakHitResult _outhit)) (Math|Rotator|MakeRotfromZ (.Normal (Collision|BreakHitResult _outhit))) "1.000000,1.000000,1.000000")))
    (Transformation|SetWorldTransform (Variables|Default|GetPreview%20Mesh) _output_get false false)
    (else
      (Development|SetHiddeninGame (Variables|Default|GetPreview%20Mesh) true false)
      (Collision|SetCollisionEnabled (Variables|Default|GetPreview%20Mesh) "NoCollision"))))

(event Custom|SetObjectToBuild
  (params (ObjectToBuild :type BPS%20Buildeable%20Structure))
  ;[0.15 0.15 0.15 0.5] Set object to build
  (bind _output_get (Variables|Default|SetBuild ObjectToBuild))
  (Components|StaticMesh|SetStaticMesh (Variables|Default|GetPreview%20Mesh) (.previemesh _output_get)))

(event Custom|Stop%20Build%20Mode
  (bind _buildtomove (Variables|Default|GetBuildToMove))
  ;[0.15 0.15 0.15 0.5] Toggle build mode
  (Variables|Default|SetInBuildMode false)
  (Variables|Default|SetIsMovingBuild false)
  (Development|SetHiddeninGame (Variables|Default|GetPreview%20Mesh) true false)
  (Collision|SetCollisionEnabled (Variables|Default|GetPreview%20Mesh) "NoCollision")
  (Utilities|IsValid _buildtomove
    (:Is%20Valid
      (Collision|SetActorEnableCollision _buildtomove true)
      (Rendering|SetActorHiddenInGame _buildtomove false)
      (Components|StaticMesh|SetStaticMesh (Variables|Default|GetPreview%20Mesh) (.previemesh (Variables|Default|GetBuild))))))

(event Custom|SetBuildToMove
  (params (BuildToMove :type Actor%20Object%20Reference) (PreviewMesh :type Static%20Mesh%20Object%20Reference))
  ;[0.15 0.15 0.15 0.5] Set build to move
  (Components|StaticMesh|SetStaticMesh (Variables|Default|GetPreview%20Mesh) PreviewMesh)
  (Variables|Default|SetBuildToMove BuildToMove)
  (Collision|SetActorEnableCollision (Variables|Default|GetBuildToMove) false)
  (Rendering|SetActorHiddenInGame (Variables|Default|GetBuildToMove) true)
  (Variables|Default|SetIsMovingBuild true)
  (CallFunction|StartBuildingMode))

(event Custom|StartBuildingMode
  ;[0.15 0.15 0.15 0.5] Toggle build mode
  (Variables|Default|SetInBuildMode true)
  (Development|SetHiddeninGame (Variables|Default|GetPreview%20Mesh) false false))

(event Custom|ToggleBuildMode
  (bind _buildtomove (Variables|Default|GetBuildToMove))
  ;[0.15 0.15 0.15 0.5] Toggle build mode
  (if (Variables|Default|GetInBuildMode)
    (Variables|Default|SetInBuildMode false)
    (Variables|Default|SetIsMovingBuild false)
    (Development|SetHiddeninGame (Variables|Default|GetPreview%20Mesh) true false)
    (Collision|SetCollisionEnabled (Variables|Default|GetPreview%20Mesh) "NoCollision")
    (Utilities|IsValid _buildtomove
      (:Is%20Valid
        (Collision|SetActorEnableCollision _buildtomove true)
        (Rendering|SetActorHiddenInGame _buildtomove false)
        (Components|StaticMesh|SetStaticMesh (Variables|Default|GetPreview%20Mesh) (.previemesh (Variables|Default|GetBuild)))))
    (else
      (Variables|Default|SetInBuildMode true)
      (Development|SetHiddeninGame (Variables|Default|GetPreview%20Mesh) false false))))

(event Custom|PlaceBuild
  ;[0.15 0.15 0.15 0.5] Place build
  (if (and (Variables|Default|GetInBuildMode) (Variables|Default|GetCanBuild))
    (if (Variables|Default|GetIsMovingBuild)
      (Transformation|SetWorldTransform (Variables|/Script/Engine.Actor|GetRootComponent (Variables|Default|GetBuildToMove)) (Variables|Default|GetBuild%20Preview%20transform) false false)
      (else
        (Game|SpawnActorfromClass (.blueprintclass (Variables|Default|GetBuild)) (Variables|Default|GetBuild%20Preview%20transform) "AdjustIfPossibleButAlwaysSpawn" "MultiplyWithRoot" 0 0)))
    (CallFunction|StopBuildMode)))

(event Custom|SetAbleToBuild
  (params (NewAble :type Boolean))
  ;[0.15 0.15 0.15 0.5] Set Able to build
  (if NewAble
    (Utilities|FlowControl|DoOnce false :!label _label
      (:Completed
        (Rendering|Material|SetMaterial (Variables|Default|GetPreview%20Mesh) 0 "/Game/Materials/PreviewMesh.PreviewMesh")
        (Development|SetHiddeninGame (Variables|Default|GetPreview%20Mesh) false false)
        (Variables|Default|SetCanBuild true)
        (goto _label_2 Reset)))
    (else
      (Utilities|FlowControl|DoOnce false :!label _label_2
        (:Completed
          (Rendering|Material|SetMaterial (Variables|Default|GetPreview%20Mesh) 0 "/Game/Materials/MI_CantBuildPreviewMaterial.MI_CantBuildPreviewMaterial")
          (Variables|Default|SetCanBuild false)
          (goto _label Reset))))))

(event EventBeginPlay
  ;[0.15 0.15 0.15 0.5] BeginPlay
  (bind _asbp_orc_player (Utilities|Casting|CastToBP_OrcPlayer (Components|GetOwner)))
  (bind _output_get (Variables|Default|SetPlayer%20BP _asbp_orc_player))
  (Variables|Default|SetCamera (Variables|/Game/Blueprint/Player/BP_OrcPlayer.BP_OrcPlayer_C|GetCamera _output_get))
  (bind _returnvalue (Game|AddComponentbyClass (Variables|Default|GetPlayer%20BP) "/Script/Engine.StaticMeshComponent" false))
  (bind _output_get_2 (Variables|Default|SetPreview%20Mesh _returnvalue))
  (Development|SetHiddeninGame _output_get_2 true false))

(event EventTick
  (params (DeltaSeconds :type Float%20%28single-precision%29))
  ;[0.15 0.15 0.15 0.5] Tick
  (if (Variables|Default|GetInBuildMode)
    (CallFunction|PreviewLoop)))

(fn SetPreviewMesh
  (bind _returnvalue (Game|AddComponentbyClass (Variables|Default|GetPlayer%20BP) "/Script/Engine.StaticMeshComponent" false (Variables|Default|GetBuild%20Preview%20transform)))
  (bind _output_get (Variables|Default|SetPreview%20Mesh _returnvalue))
  (Components|StaticMesh|SetStaticMesh _output_get "/Game/StarterContent/Props/SM_Chair.SM_Chair")
  (Collision|SetCollisionEnabled (Variables|Default|GetPreview%20Mesh) "NoCollision"))

(fn SetPreviewMeshPosition
  (params (Build%20Preview%20Location :type Vector))
  (bind _output_get (Variables|Default|SetBuild%20Preview%20transform (Math|Transform|MakeTransform Build%20Preview%20Location (Variables|Default|GetBuildPreviewRotation) "1.000000,1.000000,1.000000")))
  (Transformation|SetWorldTransform (Variables|Default|GetPreview%20Mesh) _output_get false false))