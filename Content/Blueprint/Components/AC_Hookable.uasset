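; Hookable component that holds an attached hook and pulls its object toward a target reference's object.
; Attaching parents the hook to ObjectToMove, keeping its world transform.
; Moving enables physics, then applies acceleration-based force along the direction from GetDirection in a retriggerable-delay loop.
; The loop ends when close to the target or past an iteration cap, then zeroes velocity and disables physics.
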(event EventBeginPlay)

(event EventTick
  (params (DeltaSeconds :type Float%20%28single-precision%29)))

(event EventFNAttachHook
  (params (HookToAttach :type BP%20Hook%20Object%20Reference))
  (Transformation|AttachComponentToComponent HookToAttach (Variables|Default|GetObjectToMove) "None" "KeepWorld" "KeepWorld" "KeepWorld" false)
  (Variables|Default|SetHook%20to%20Attach HookToAttach))

(event EventFnMovetoTarge
  (params (TargetReference :type AC%20Hookable%20Object%20Reference))
  (Variables|Default|SetTargetRef TargetReference)
  (Physics|SetSimulatePhysics (Variables|Default|GetObjectToMove) true)
  (Variables|Default|SetIterations 0)
  (bind (_returnvalue _returnvalue1) (CallFunction|GetDirection :!label _label))
  (if (and (> _returnvalue1 1e+02) (>= (Variables|Default|GetMaxIterations) (Variables|Default|GetIterations)))
    (Physics|AddForce (Variables|Default|GetObjectToMove) _returnvalue "None" true)
    (Math|Integer|IncrementInt (Variables|Default|GetIterations)
      (:%20%20
        (Utilities|FlowControl|RetriggerableDelay 0.2)
        (goto _label)))
    (else
      (Development|PrintString "Exit")
      (Physics|SetPhysicsLinearVelocity (Variables|Default|GetObjectToMove) "0, 0, 0" false "None")
      (Physics|SetSimulatePhysics (Variables|Default|GetObjectToMove) false))))

(fn GetDirection
  (bind _objecttomove (Variables|Default|GetObjectToMove))
  (bind _targetref (Variables|Default|GetTargetRef))
  (bind _returnvalue (Transformation|GetWorldLocation _objecttomove))
  (bind _objecttomove_2 (Variables|AC_Hookable_C|GetObjectToMove _targetref))
  (bind _returnvalue_2 (Transformation|GetWorldLocation _objecttomove_2))
  (return (* (Math|Vector|Normalize (Math|Vector|GetUnitDirection(Vector) _returnvalue _returnvalue_2)) (Variables|Default|GetSpeed)) (Math|Vector|Distance(Vector) _returnvalue _returnvalue_2)))