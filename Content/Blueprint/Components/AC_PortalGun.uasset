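; AC_PortalGun is an actor component that lets its owner shoot linked orange and blue portals onto surfaces.
; On BeginPlay it spawns both portals hidden and without collision, links them to each other and caches the owner's camera.
; Right and left shoot inputs trace from the camera, with persistent debug drawing.
; A hit on a "Portal"-tagged actor places and activates that portal along the surface normal; otherwise it is disabled and hidden.
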(event Input|EnhancedActionEvents|EnhancedInputActionIA_RightShoot
  (params (ActionValue :type Boolean) (ElapsedSeconds :type Float%20%28double-precision%29) (TriggeredSeconds :type Float%20%28double-precision%29) (InputAction :type Input%20Action%20Object%20Reference :default "/Game/FirstPerson/Input/Actions/IA_RightShoot.IA_RightShoot"))
  (:Started
    (CallFunction|MovePortal (Variables|Default|GetBP_OrangePortal))))

(event Input|EnhancedActionEvents|EnhancedInputActionIA_LeftShoot
  (params (ActionValue :type Boolean) (ElapsedSeconds :type Float%20%28double-precision%29) (TriggeredSeconds :type Float%20%28double-precision%29) (InputAction :type Input%20Action%20Object%20Reference :default "/Game/FirstPerson/Input/Actions/IA_LeftShoot.IA_LeftShoot"))
  (:Started
    (CallFunction|MovePortal (Variables|Default|GetBP_BluePortal))))

(event EventBeginPlay
  (bind _returnvalue (Game|SpawnActorfromClass "/Game/Blueprint/Objects/Portals/BP_Portal_Orange.BP_Portal_Orange_C" (Math|Transform|MakeTransform "0, 0, 0" "0, 0, 0" "1.000000,1.000000,1.000000") "AdjustIfPossibleButAlwaysSpawn" "MultiplyWithRoot" 0 0))
  (bind _output_get (Variables|Default|SetBP_OrangePortal _returnvalue))
  (Collision|SetActorEnableCollision _output_get false)
  (Rendering|SetActorHiddenInGame _output_get true)
  (bind _returnvalue_2 (Game|SpawnActorfromClass "/Game/Blueprint/Objects/Portals/BP_Portal_Blue.BP_Portal_Blue_C" (Math|Transform|MakeTransform "0, 0, 0" "0, 0, 0" "1.000000,1.000000,1.000000") "AdjustIfPossibleButAlwaysSpawn" "MultiplyWithRoot" 0 0))
  (bind _output_get_2 (Variables|Default|SetBP_BluePortal _returnvalue_2))
  (Collision|SetActorEnableCollision _output_get_2 false)
  (Rendering|SetActorHiddenInGame _output_get_2 true)
  (Variables|Default|SetCameraRef (Actor|GetComponentbyClass (Components|GetOwner) "/Script/Engine.CameraComponent"))
  (Variables|/Game/Blueprint/Objects/Portals/BP_Portal.BP_Portal_C|SetOtherPortal (Variables|Default|GetBP_OrangePortal) (Variables|Default|GetBP_BluePortal))
  (Variables|/Game/Blueprint/Objects/Portals/BP_Portal.BP_Portal_C|SetOtherPortal (Variables|Default|GetBP_BluePortal) (Variables|Default|GetBP_OrangePortal)))

(fn MovePortal
  (params (PortalToMove :type BP%20Portal%20Object%20Reference))
  (bind _cameraref (Variables|Default|GetCameraRef))
  (bind _returnvalue (Transformation|GetWorldLocation _cameraref))
  (bind (_outhit _returnvalue_2) (Collision|LineTraceByChannel _returnvalue (+ _returnvalue (* (Math|Vector|GetForwardVector _cameraref) (Variables|Default|GetRayDistance))) "TraceTypeQuery1" false 0 "Persistent"))
  (if _returnvalue_2
    (if (Actor|ActorHasTag (.HitActor (Collision|BreakHitResult _outhit)) "Portal")
      (Rendering|SetActorHiddenInGame PortalToMove true)
      (Transformation|SetActorTransform PortalToMove (Math|Transform|MakeTransform (.Location (Collision|BreakHitResult _outhit)) (Math|Rotator|MakeRotfromZ (.Normal (Collision|BreakHitResult _outhit))) "1.000000,1.000000,1.000000") false true)
      (Variables|/Game/Blueprint/Objects/Portals/BP_Portal.BP_Portal_C|SetIsReady PortalToMove true)
      (Collision|SetActorEnableCollision PortalToMove true)
      (Rendering|SetActorHiddenInGame PortalToMove false)
      (else
        (Variables|/Game/Blueprint/Objects/Portals/BP_Portal.BP_Portal_C|SetIsReady PortalToMove false :!label _label)
        (Collision|SetActorEnableCollision PortalToMove false)
        (Rendering|SetActorHiddenInGame PortalToMove true)))
    (else
      (goto _label))))