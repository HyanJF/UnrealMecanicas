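; AC_Movable is an actor component that lets its owner be relocated or upgraded through the trap-building system.
; Move finds the target's AC_TrapBuilder and passes it the owner and a preview mesh via SetBuildToMove.
; Interaction casts the given actor to BP_OrcPlayer and calls ShowUpgrade with its BPBuildeable.
; Both functions return whether they succeeded, and the component runs no event logic of its own.
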(event EventBeginPlay)

(event EventTick
  (params (DeltaSeconds :type Float%20%28single-precision%29)))

(fn Move
  (params (Target :type Actor%20Object%20Reference))
  (bind _returnvalue (Actor|GetComponentbyClass Target "/Game/Blueprint/Components/AC_TrapBuilder.AC_TrapBuilder_C"))
  (Utilities|IsValid _returnvalue
    (:Is%20Valid
      (Default|SetBuildtoMove _returnvalue (Components|GetOwner) (Variables|Default|GetPreview%20Mesh))
      (return true))
    (:Is%20Not%20Valid
      (return false))))

(fn Interaction
  (params (ActorT :type Actor%20Object%20Reference))
  (bind _asbp_orc_player (Utilities|Casting|CastToBP_OrcPlayer ActorT)
    (:then
      (Default|ShowUpgrade _asbp_orc_player (Variables|Default|GetBP_Buildeable))
      (return true))
    (:CastFailed
      (return false))))