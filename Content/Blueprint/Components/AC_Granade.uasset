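; Actor component that lets its owner aim and throw grenades through the IA_Granade Enhanced Input action.
; While the action triggers, it draws a one-frame predicted projectile path from the owner's camera along its forward vector.
; On completion, it spawns a Granade actor at the camera and applies a velocity-change impulse to its Sphere, using the preview's launch velocity.
; The scene component cached at BeginPlay is unused.
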(event Input|EnhancedActionEvents|EnhancedInputActionIA_Granade
  (params (ActionValue :type Boolean) (ElapsedSeconds :type Float%20%28double-precision%29) (TriggeredSeconds :type Float%20%28double-precision%29) (InputAction :type Input%20Action%20Object%20Reference :default "/Game/FirstPerson/Input/Actions/IA_Granade.IA_Granade"))
  (bind _camera (Variables|Default|GetCamera))
  (:Triggered
    (Class|GameplayStatics|BlueprintPredictProjectilePathAdvanced (Utilities|Struct|MakePredictProjectilePathParams (Transformation|GetWorldLocation _camera) (* (Math|Vector|GetForwardVector _camera) 1e+03) true 1e+01 1.0 true "ECC_WorldStatic" "ObjectTypeQuery1" (Utilities|Array|MakeArray (Components|GetOwner)) 2e+01 0.0 "ForOneFrame" 5.0 false)))
  (:Completed
    (bind _returnvalue (Game|SpawnActorfromClass "/Game/Blueprint/Explosives/Granade.Granade_C" (Transformation|GetWorldTransform _camera) "Undefined" "MultiplyWithRoot" (Components|GetOwner) 0))
    (Physics|AddImpulse (Variables|/Game/Blueprint/Explosives/Granade.Granade_C|GetSphere _returnvalue) (* (Math|Vector|GetForwardVector (Variables|Default|GetCamera)) 1e+03) "None" true)))

(event EventBeginPlay
  (bind _returnvalue (Components|GetOwner))
  (Variables|Default|SetCamera (Actor|GetComponentbyClass _returnvalue "/Script/Engine.CameraComponent"))
  (Variables|Default|SetSpawn (Actor|GetComponentbyClass _returnvalue "/Script/Engine.SceneComponent")))