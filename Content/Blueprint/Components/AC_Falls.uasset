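; Actor component that gives its owning character a glide while falling, driven by the IA_Plane input action.
; It caches the owner's CharacterMovementComponent on BeginPlay.
; Pressing the input mid-fall lowers gravity scale and raises max walk speed.
; Releasing it, or pressing while not falling, sets both back to fixed normal values; landing alone does not reset them.
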(event Input|EnhancedActionEvents|EnhancedInputActionIA_Plane
  (params (ActionValue :type Boolean) (ElapsedSeconds :type Float%20%28double-precision%29) (TriggeredSeconds :type Float%20%28double-precision%29) (InputAction :type Input%20Action%20Object%20Reference :default "/Game/FirstPerson/Input/Actions/IA_Plane.IA_Plane"))
  (bind _move (Variables|Default|GetMove))
  (bind _move_2 (Variables|Default|GetMove))
  (:Started
    (if (AI|Components|NavMovement|IsFalling (Variables|Default|GetMove))
      (Variables|/Script/Engine.CharacterMovementComponent|SetGravityScale _move_2 0.25)
      (Variables|/Script/Engine.CharacterMovementComponent|SetMaxWalkSpeed _move_2 7e+02)
      (else
        (Variables|/Script/Engine.CharacterMovementComponent|SetGravityScale _move 1.0 :!label _label)
        (Variables|/Script/Engine.CharacterMovementComponent|SetMaxWalkSpeed _move 6e+02))))
  (:Completed
    (goto _label)))

(event EventBeginPlay
  (Variables|Default|SetMove (Actor|GetComponentbyClass (Components|GetOwner) "/Script/Engine.CharacterMovementComponent")))