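; Actor component that lets its owner interact with objects in the world through the IA_Interact input.
; On BeginPlay it caches the owner's camera; on each press it line-traces forward from it on the Visibility channel up to RayDistance.
; On a hit, it calls Interaction on the hit actor's first component implementing BPI_Interaction, passing the owner, and prints the returned value.
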(event Input|EnhancedActionEvents|EnhancedInputActionIA_Interact
  (params (ActionValue :type Boolean) (ElapsedSeconds :type Float%20%28double-precision%29) (TriggeredSeconds :type Float%20%28double-precision%29) (InputAction :type Input%20Action%20Object%20Reference :default "/Game/FirstPerson/Input/Actions/IA_Interact.IA_Interact"))
  (bind _camera (Variables|Default|GetCamera))
  (bind _returnvalue (Transformation|GetWorldTransform _camera))
  ;[0.15 0.15 0.15 0.5] InteractionObject
  (:Started
    (Variables|Default|SetInteracted false)
    (bind (_outhit _returnvalue_2) (Collision|LineTraceByChannel (.location _returnvalue) (+ (.location _returnvalue) (* (Math|Vector|GetForwardVector (.rotation _returnvalue)) (Variables|Default|GetRayDistance))) "TraceTypeQuery1" false 0 "None" true "(R=1.000000,G=0.000000,B=0.390478,A=1.000000)" "(R=0.576232,G=1.000000,B=0.000000,A=1.000000)"))
    (if _returnvalue_2
      (if (not (Variables|Default|GetInteracted))
        (bind _asbpi_interaction (Utilities|Casting|CastToBPI_Interaction (Utilities|Array|Get(acopy) (Class|Actor|GetComponentsbyInterface (.HitActor (Collision|BreakHitResult _outhit)) "/Game/Blueprint/Interface/BPI_Interaction.BPI_Interaction_C"))))
        (Variables|Default|SetInteracted true)
        (bind _iscompleted (Default|Interaction _asbpi_interaction (Components|GetOwner)))
        (Development|PrintText (Utilities|Text|FormatText (Utilities|Text|ToText(Boolean) _iscompleted)) true true "(R=1.000000,G=0.000000,B=0.942791,A=1.000000)")))))

(event EventBeginPlay
  ;[0.15 0.15 0.15 0.5] BeginPlay
  (Variables|Default|SetCamera (Actor|GetComponentbyClass (Components|GetOwner) "/Script/Engine.CameraComponent")))