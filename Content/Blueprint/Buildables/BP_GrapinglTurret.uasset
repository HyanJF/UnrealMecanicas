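; Grappling turret buildable that hooks enemies with hookable components, damages them and pulls two of them toward each other.
; An overlap volume tracks targets, and successive TryAttack calls line-trace to attach pre-spawned yellow and purple hooks to the first two.
; Once both points are set, it triggers the mutual pull, hides the hooks and retries after HitDelay.
; Upgrade 1 shortens the hit delay and Upgrade 2 scales damage.
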(event OnComponentBeginOverlap(EnemyDetection)
  (params (OverlappedComponent :type Primitive%20Component%20Object%20Reference) (OtherActor :type Actor%20Object%20Reference) (OtherComp :type Primitive%20Component%20Object%20Reference) (OtherBodyIndex :type Integer) (bFromSweep :type Boolean) (SweepResult :type Hit%20Result%20Structure%20%28by%20ref%29))
  (bind _returnvalue (Actor|GetComponentbyClass OtherActor "/Game/Blueprint/Components/AC_Hookable.AC_Hookable_C"))
  (Utilities|IsValid _returnvalue
    (:Is%20Valid
      (Utilities|Array|AddUnique (Variables|Default|GetHookableEnemies) _returnvalue))))

(event OnComponentEndOverlap(EnemyDetection)
  (params (OverlappedComponent :type Primitive%20Component%20Object%20Reference) (OtherActor :type Actor%20Object%20Reference) (OtherComp :type Primitive%20Component%20Object%20Reference) (OtherBodyIndex :type Integer))
  (Utilities|Array|RemoveItem (Variables|Default|GetHookableEnemies) (Actor|GetComponentbyClass OtherActor "/Game/Blueprint/Components/AC_Hookable.AC_Hookable_C")))

(event Custom|TryAttack
  ;[0.15 0.15 0.15 0.5] Move
  (if (> (Utilities|Array|Length (Variables|Default|GetHookableEnemies)) 0)
    (Utilities|IsValid (Variables|Default|GetFirst_Point)
      (:Is%20Valid
        (if (Utilities|Array|IsValidIndex (Variables|Default|GetHookableEnemies) 1)
          (bind _hookedactor (CallFunction|MoveHook (Variables|Default|GetPurpleHook) (Utilities|Array|Get(acopy) (Variables|Default|GetHookableEnemies) 1)))
          (bind _output_get (Variables|Default|SetSecond_Point _hookedactor))
          (if (and (Utilities|IsValid _output_get) (Utilities|IsValid (stale _output_get_2))) :!label _label
            (Default|FnMovetoTarge (Variables|Default|GetFirst_Point) (Variables|Default|GetSecond_Point))
            (Default|FnMovetoTarge (Variables|Default|GetSecond_Point) (Variables|Default|GetFirst_Point))
            (Variables|Default|SetFirst_Point 0)
            (Variables|Default|SetSecond_Point 0)
            (Utilities|FlowControl|Delay 1.0)
            (Rendering|SetActorHiddenInGame (Variables|Default|GetPurpleHook) true)
            (Rendering|SetActorHiddenInGame (Variables|Default|GetYellowHook) true)
            (Utilities|FlowControl|Delay (Variables|Default|GetHitDelay))
            (CallFunction|TryAttack))))
      (:Is%20Not%20Valid
        (bind _hookedactor_2 (CallFunction|MoveHook (Variables|Default|GetYellowHook) (Utilities|Array|Get(acopy) (Variables|Default|GetHookableEnemies))))
        (bind _output_get_2 (Variables|Default|SetFirst_Point _hookedactor_2))
        (goto _label)))))

(event EventBeginPlay
  (|CallParentFunction)
  (bind _returnvalue (Game|SpawnActorfromClass "/Game/Blueprint/Objects/Hook/BP_Hook_Purple.BP_Hook_Purple_C" (Math|Transform|MakeTransform "0, 0, 0" "0, 0, 0" "1.000000,1.000000,1.000000") "Undefined" "MultiplyWithRoot" 0 0))
  (bind _output_get (Variables|Default|SetPurpleHook _returnvalue))
  (Rendering|SetActorHiddenInGame _output_get true)
  (bind _returnvalue_2 (Game|SpawnActorfromClass "/Game/Blueprint/Objects/Hook/BP_Hook_Yellow.BP_Hook_Yellow_C" (Math|Transform|MakeTransform "0, 0, 0" "0, 0, 0" "1.000000,1.000000,1.000000") "Undefined" "MultiplyWithRoot" 0 0))
  (bind _output_get_2 (Variables|Default|SetYellowHook _returnvalue_2))
  (Rendering|SetActorHiddenInGame _output_get_2 true)
  (CallFunction|SetUpdate1)
  (CallFunction|SetUpdate2))

(event Collision|EventActorBeginOverlap
  (params (OtherActor :type Actor%20Object%20Reference))
  (|CallParentFunction OtherActor) ; This node is disabled and will not be called.\nDrag off pins to build functionality.
)

(event EventTick
  (params (DeltaSeconds :type Float%20%28single-precision%29))
  (|CallParentFunction DeltaSeconds) ; This node is disabled and will not be called.\nDrag off pins to build functionality.
)

(event EventUpgrade2
  (Variables|Default|SetUpgrade2Level (+ (Variables|Default|GetUpgrade2Level) 1))
  (CallFunction|SetUpdate2))

(event EventUpgrade1
  (Variables|Default|SetUpgrade1Level (+ (Variables|Default|GetUpgrade1Level) 1))
  (CallFunction|SetUpdate1))

(fn ConstructionScript
  (|CallParentFunction))

(fn MoveHook
  (params (Hook :type BP%20Hook%20Object%20Reference) (EnemieToHook :type AC%20Hookable%20Object%20Reference))
  (bind _objecttomove (Variables|/Game/Blueprint/Components/AC_Hookable.AC_Hookable_C|GetObjectToMove EnemieToHook))
  (bind _returnvalue (Transformation|GetWorldLocation _objecttomove))
  (bind _returnvalue_2 (Components|GetOwner EnemieToHook))
  (bind _returnvalue_3 (Actor|GetComponentbyClass _returnvalue_2 "/Game/Blueprint/Components/AC_Damagable.AC_Damagable_C"))
  (bind (_outhit _returnvalue_4) (Collision|LineTraceByChannel (Transformation|GetWorldLocation (Variables|Default|GetObjectMesh)) (Math|Vector|MakeVector (.x _returnvalue) (.y _returnvalue) (.z _returnvalue)) "TraceTypeQuery1" false 0 "ForDuration" true "(R=1.000000,G=0.000000,B=0.000000,A=1.000000)" "(R=0.000000,G=1.000000,B=0.000000,A=1.000000)" 0.5))
  (if _returnvalue_4
    (Rendering|SetActorHiddenInGame Hook true)
    (Transformation|SetActorTransform Hook (Math|Transform|MakeTransform (.Location (Collision|BreakHitResult _outhit)) (Math|Rotator|MakeRotfromZ (.Normal (Collision|BreakHitResult _outhit))) "1.000000,1.000000,1.000000") false true)
    (Default|FNAttachHook EnemieToHook Hook)
    (Rendering|SetActorHiddenInGame Hook false)
    (Utilities|IsValid _returnvalue_3
      (:Is%20Valid
        (Default|FnDamage _returnvalue_3 self (Variables|Default|GetDamage)))
      (:Is%20Not%20Valid
        _))
    (return EnemieToHook)
    (else
      (Transformation|DetachFromActor Hook "KeepRelative" "KeepRelative" "KeepRelative")
      (Rendering|SetActorHiddenInGame Hook true))))

(fn GetUpgrade2
  (return (Utilities|Struct|MakeBPS_Stat "" 0 0.0 0)))

(fn SetUpdate1
  (|CallParentFunction)
  (Variables|Default|SetHitDelay (Math|Float|Max(Float) (- (Variables|Default|GetBaseHitDelay) (- (Variables|Default|GetUpgrade1Level) 0.25)) 0.2)))

(fn SetUpdate2
  (|CallParentFunction)
  (Variables|Default|SetDamage (+ (Variables|Default|GetBaseDamage) (* (Variables|Default|GetBaseDamage) (* (Variables|Default|GetUpgrade2Level) 0.5)))))