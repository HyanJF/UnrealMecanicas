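; BP_Buildable looks like a base Blueprint for buildable objects with two upgradeable stats.
; On BeginPlay it registers itself with its ACMovable reference.
; Getters expose both stats and their upgrade prices, which rise linearly by half the base price per level.
; Upgrade and the two SetUpdate functions are empty, and Interaction returns false, apparently as defaults for child classes to override.
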(event EventBeginPlay
  (Variables|/Game/Blueprint/Components/AC_Upgradeable.AC_Upgradeable_C|SetBP_Buildeable (Variables|Default|GetAC_Movable) self))

(fn ConstructionScript)

(fn Upgrade
  (params (Stat :type BPS%20Stat%20Structure)))

(fn GetPrice1
  (return (+ (Variables|Default|GetUpgrade1Price) (* (Variables|Default|GetUpgrade1Price) (* (Variables|Default|GetUpgrade1Level) 0.5)))))

(fn GetPrice2
  (bind _upgrade2price (Variables|Default|GetUpgrade2Price))
  (return (+ _upgrade2price (* _upgrade2price (* (Variables|Default|GetUpgrade2Level) 0.5)))))

(fn SetUpdate1)

(fn SetUpdate2)

(fn GetUpgrade1
  (return (Variables|Default|GetStat1)))

(fn GetUpgrade2
  (return (Variables|Default|GetStat2)))

(fn Interaction
  (params (ActorT :type Actor%20Object%20Reference))
  (return false))