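; Slow trap buildable that reduces the walk speed of characters tagged Enemy while they overlap its InteractionDetection component.
; Begin overlap subtracts SpeedReduction from MaxWalkSpeed and end overlap is meant to add it back.
; Two upgrade tracks scale capped SpeedReduction and Damage from base values, though Damage is not applied here.
; Both are computed at BeginPlay through parent-extending functions; upgrade events here only increment their levels.
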(event OnComponentEndOverlap(InteractionDetection)
  (params (OverlappedComponent :type Primitive%20Component%20Object%20Reference) (OtherActor :type Actor%20Object%20Reference) (OtherComp :type Primitive%20Component%20Object%20Reference) (OtherBodyIndex :type Integer))
  (if (Actor|ActorHasTag OtherActor "Enemy")
    (bind _ascharacter (Utilities|Casting|CastToCharacter 0))
    (Variables|/Script/Engine.CharacterMovementComponent|SetMaxWalkSpeed (Variables|/Script/Engine.Character|GetCharacterMovement _ascharacter) (+ (Variables|/Script/Engine.CharacterMovementComponent|GetMaxWalkSpeed (Variables|/Script/Engine.Character|GetCharacterMovement _ascharacter)) (Variables|Default|GetSpeedReduction)))))

(event OnComponentBeginOverlap(InteractionDetection)
  (params (OverlappedComponent :type Primitive%20Component%20Object%20Reference) (OtherActor :type Actor%20Object%20Reference) (OtherComp :type Primitive%20Component%20Object%20Reference) (OtherBodyIndex :type Integer) (bFromSweep :type Boolean) (SweepResult :type Hit%20Result%20Structure%20%28by%20ref%29))
  (Development|PrintString (Utilities|GetDisplayName OtherActor))
  (if (Actor|ActorHasTag OtherActor "Enemy")
    (bind _ascharacter (Utilities|Casting|CastToCharacter OtherActor))
    (Variables|/Script/Engine.CharacterMovementComponent|SetMaxWalkSpeed (Variables|/Script/Engine.Character|GetCharacterMovement _ascharacter) (- (Variables|/Script/Engine.CharacterMovementComponent|GetMaxWalkSpeed (Variables|/Script/Engine.Character|GetCharacterMovement _ascharacter)) (Variables|Default|GetSpeedReduction)))))

(event EventBeginPlay
  (|CallParentFunction)
  (CallFunction|SetUpdate1)
  (CallFunction|SetUpdate2))

(event Collision|EventActorBeginOverlap
  (params (OtherActor :type Actor%20Object%20Reference)))

(event EventTick
  (params (DeltaSeconds :type Float%20%28single-precision%29)))

(event EventUpgrade1
  (Variables|Default|SetUpgrade1Level (+ (Variables|Default|GetUpgrade1Level) 1)))

(event EventUpgrade2
  (Variables|Default|SetUpgrade2Level (+ (Variables|Default|GetUpgrade2Level) 1)))

(fn ConstructionScript
  (|CallParentFunction))

(fn SetUpdate1
  (bind _basespeedreduction (Variables|Default|GetBaseSpeedReduction))
  (|CallParentFunction)
  (Variables|Default|SetSpeedReduction (Math|Float|Min(Float) 5e+02 (+ _basespeedreduction (* _basespeedreduction (* (Variables|Default|GetUpgrade1Level) 0.5))))))

(fn SetUpdate2
  (bind _basedamage (Variables|Default|GetBaseDamage))
  (|CallParentFunction)
  (Variables|Default|SetDamage (+ _basedamage (* _basedamage (* (Variables|Default|GetUpgrade2Level) 0.5)))))