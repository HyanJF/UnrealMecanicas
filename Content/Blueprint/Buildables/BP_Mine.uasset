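; BP_Mine is a buildable mine that damages actors entering its InteractionDetection component through BPI_Damagable, crediting the player controller.
; Each hit starts a HitDelay cooldown, and overlaps that begin during it are ignored.
; Two upgrade events raise level counters, which the SetUpdate overrides use to shorten the delay, down to a minimum, and scale damage linearly from its base.
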(event OnComponentBeginOverlap(InteractionDetection)
  (params (OverlappedComponent :type Primitive%20Component%20Object%20Reference) (OtherActor :type Actor%20Object%20Reference) (OtherComp :type Primitive%20Component%20Object%20Reference) (OtherBodyIndex :type Integer) (bFromSweep :type Boolean) (SweepResult :type Hit%20Result%20Structure%20%28by%20ref%29))
  (bind _returnvalue (Game|GetPlayerController 0))
  (if (!= OtherActor _returnvalue)
    (if (Variables|Default|GetIsReadyToAttack)
      (bind _asbpi_damagable (Utilities|Casting|CastToBPI_Damagable OtherActor))
      (Default|FnDamage _asbpi_damagable _returnvalue (Variables|Default|GetDamage))
      (Variables|Default|SetIsReadyToAttack false)
      (Utilities|FlowControl|Delay (Variables|Default|GetHitDelay))
      (Variables|Default|SetIsReadyToAttack true))))

(event EventBeginPlay
  (|CallParentFunction))

(event Collision|EventActorBeginOverlap
  (params (OtherActor :type Actor%20Object%20Reference))
  (|CallParentFunction OtherActor) ; This node is disabled and will not be called.\nDrag off pins to build functionality.
)

(event EventTick
  (params (DeltaSeconds :type Float%20%28single-precision%29))
  (|CallParentFunction DeltaSeconds) ; This node is disabled and will not be called.\nDrag off pins to build functionality.
)

(event EventUpgrade1
  (Variables|Default|SetUpgrade1Level (+ (Variables|Default|GetUpgrade1Level) 1)))

(event EventUpgrade2
  (Variables|Default|SetUpgrade2Level (+ (Variables|Default|GetUpgrade2Level) 1)))

(fn ConstructionScript
  (|CallParentFunction))

(fn SetUpdate1
  (|CallParentFunction)
  (Variables|Default|SetHitDelay (Math|Float|Max(Float) (- (Variables|Default|GetBaseHitDelay) (- (Variables|Default|GetUpgrade1Level) 0.25)) 0.2)))

(fn SetUpdate2
  (|CallParentFunction)
  (Variables|Default|SetDamage (+ (Variables|Default|GetBaseDamage) (* (Variables|Default|GetBaseDamage) (* (Variables|Default|GetUpgrade2Level) 0.5)))))