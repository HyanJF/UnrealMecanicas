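; Buildable portal trap that teleports nearby actors tagged Teleportable to a linked BP_PortalExit, which it spawns beside itself on BeginPlay.
; A tagged overlap disables and hides the portal, then a debug-drawn sphere trace moves every tagged hit to the exit.
; The portal re-arms after a cooldown, only if the trace hit something.
; Upgrade levels widen the radius and shorten the cooldown, with crossed naming: SetUpgrade1 reads Upgrade2Level and vice versa.
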(event OnComponentBeginOverlap(PortalEffect)
  (params (OverlappedComponent :type Primitive%20Component%20Object%20Reference) (OtherActor :type Actor%20Object%20Reference) (OtherComp :type Primitive%20Component%20Object%20Reference) (OtherBodyIndex :type Integer) (bFromSweep :type Boolean) (SweepResult :type Hit%20Result%20Structure%20%28by%20ref%29))
  (bind _portaleffect (Variables|Default|GetPortalEffect))
  (bind _returnvalue (Transformation|GetWorldLocation _portaleffect))
  (if (and (Variables|Default|GetCanTP) (Actor|ActorHasTag OtherActor "Teleportable"))
    (Variables|Default|SetCanTP false)
    (Collision|SetCollisionEnabled (Variables|Default|GetPortalEffect) "NoCollision")
    (Development|SetHiddeninGame (Variables|Default|GetPortalEffect) true false)
    (bind (_outhits _returnvalue_2) (Collision|MultiSphereTraceByChannel _returnvalue _returnvalue (Variables|Default|GetRadius) "TraceTypeQuery1" false 0 "ForDuration"))
    (if _returnvalue_2
      (for _array_element _outhits
        (if (Actor|ActorHasTag (.HitActor (Collision|BreakHitResult _array_element)) "Teleportable")
          (Transformation|SetActorLocation (.HitActor (Collision|BreakHitResult _array_element)) (Transformation|GetWorldLocation (Variables|/Game/Blueprint/Buildables/BP_PortalExit.BP_PortalExit_C|GetExitPoint (Variables|Default|GetExit))) false false)))
      (Utilities|FlowControl|Delay (Variables|Default|GetCooldown))
      (Variables|Default|SetCanTP true)
      (Development|SetHiddeninGame (Variables|Default|GetPortalEffect) false false)
      (Collision|SetCollisionEnabled (Variables|Default|GetPortalEffect) "QueryOnly"))))

(event EventBeginPlay
  (bind _objectmesh (Variables|Default|GetObjectMesh))
  (bind _returnvalue (Transformation|GetWorldTransform _objectmesh))
  (|CallParentFunction)
  (bind _returnvalue_2 (Game|SpawnActorfromClass "/Game/Blueprint/Buildables/BP_PortalExit.BP_PortalExit_C" (Math|Transform|MakeTransform (+ (.location _returnvalue) "250.000000,0.000000,0.000000") (.rotation _returnvalue) (.scale _returnvalue)) "AdjustIfPossibleButAlwaysSpawn" "MultiplyWithRoot" 0 0))
  (Variables|Default|SetExit _returnvalue_2))

(event EventUpgrade2
  (Variables|Default|SetUpgrade2Level (+ (Variables|Default|GetUpgrade2Level) 1)))

(event EventUpgrade1
  (Variables|Default|SetUpgrade1Level (+ (Variables|Default|GetUpgrade1Level) 1)))

(fn ConstructionScript
  (|CallParentFunction))

(fn SetUpgrade)

(fn GetUpgrade2
  (return ""))

(fn SetUpgrade1
  (Variables|Default|SetCooldown (Math|Float|Max(Float) (- (Variables|Default|GetBaseCooldown) (* (Variables|Default|GetUpgrade2Level) 0.2)) 0.2)))

(fn SetUpgrade2
  (Variables|Default|SetRadius (+ (Variables|Default|GetBaseRadius) (* (Variables|Default|GetUpgrade1Level) 5e+01))))