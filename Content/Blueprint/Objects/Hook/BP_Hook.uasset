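; BP_Hook is a hook actor that moves its Cone component toward a target, by physics force or by interpolation.
; StartMove pushes the Cone toward the target every half second, with force scaled by the starting distance.
; That distance is never recomputed in the loop, so the actor self-destructs only if it starts within 0.1 units.
; A separate Move event interpolates the Cone to another hook's Cone world transform using MoveComponentTo, which takes relative values.
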(event Custom|StartMove
  (params (Target :type Actor%20Object%20Reference))
  (bind _returnvalue (Transformation|GetActorLocation))
  (bind _returnvalue_2 (Transformation|GetActorLocation Target))
  (Variables|Default|SetTarget Target)
  (bind _output_get (Variables|Default|SetDistance (Math|Vector|Distance(Vector) _returnvalue_2 _returnvalue)))
  (Physics|AddForce (Variables|Default|GetCone) (* _output_get (Math|Vector|Normalize (- _returnvalue_2 _returnvalue))) "None" false :!label _label)
  (Utilities|FlowControl|Delay 0.5)
  (if (> (Variables|Default|GetDistance) 0.1)
    (goto _label)
    (else
      (Actor|DestroyActor))))

(event Custom|Move
  (params (HookTargetr :type BP%20Hook%20Object%20Reference))
  (bind _cone (Variables|BP_Hook_C|GetCone HookTargetr))
  (Components|MoveComponentTo (Variables|Default|GetCone) (Transformation|GetWorldLocation _cone) (Transformation|GetWorldRotation _cone) false false 5.0 false))

(fn ConstructionScript)