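; BP_HookableBox is a box object that a hook can attach to.
; FNAttachHook attaches the given hook component to the box's StaticMesh, keeping its world transform.
; GetDirection returns a speed-scaled direction and the distance to TargetRef's mesh.
; An iteration-capped force loop would pull the box toward that target, but it is disconnected and FnMovetoTarge is empty, so the box never moves itself.
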(event EventFnMovetoTarge
  (params (TargetReference :type AC%20Hookable%20Object%20Reference)))

(event EventFNAttachHook
  (params (HookToAttach :type BP%20Hook%20Object%20Reference))
  (Transformation|AttachComponentToComponent HookToAttach (Variables|Default|GetStaticMesh) "None" "KeepWorld" "KeepWorld" "KeepWorld" true)
  (Variables|Default|SetHook%20to%20Attach HookToAttach))

(fn ConstructionScript)

(fn GetDirection
  (bind _staticmesh (Variables|Default|GetStaticMesh))
  (bind _targetref (Variables|Default|GetTargetRef))
  (bind _returnvalue (Transformation|GetWorldLocation _staticmesh))
  (bind _staticmesh_2 (Variables|BP_HookableBox_C|GetStaticMesh _targetref))
  (bind _returnvalue_2 (Transformation|GetWorldLocation _staticmesh_2))
  (return (* (Math|Vector|Normalize (Math|Vector|GetUnitDirection(Vector) _returnvalue _returnvalue_2)) (Variables|Default|GetSpeed)) (Math|Vector|Distance(Vector) _returnvalue _returnvalue_2)))