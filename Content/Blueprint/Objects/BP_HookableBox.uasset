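; BP_HookableBox is a physics box that hooks can attach to and that can be pulled toward a target object.
; FnMovetoTarge loops on a short retriggerable delay, adding mass-independent force along GetDirection's speed-scaled vector toward the target's mesh.
; The pull stops once the box is close enough or the iteration cap is exceeded.
; FNAttachHook attaches a given hook component to the static mesh, keeping its world transform.
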(event EventFnMovetoTarge
  (params (TargetReference :type BP%20Hookable%20Box%20Object%20Reference))
  (Variables|Default|SetTargetRef TargetReference)
  (bind (_direction _distance) (CallFunction|GetDirection :!label _label))
  (if (and (> _distance 1.5e+02) (>= (Variables|Default|GetMaxIterations) (Variables|Default|GetIterations)))
    (Physics|AddForce (Variables|Default|GetStaticMesh) _direction "None" true)
    (Math|Integer|IncrementInt (Variables|Default|GetIterations)
      (:%20%20
        (Utilities|FlowControl|RetriggerableDelay 0.2)
        (goto _label)))
    (else
      (Development|PrintString "Exit"))))

(event EventFNAttachHook
  (params (HookToAttach :type BP%20Hook%20Object%20Reference))
  (Transformation|AttachComponentToComponent HookToAttach (Variables|Default|GetStaticMesh) "None" "KeepWorld" "KeepWorld" "KeepWorld" true))

(fn ConstructionScript)

(fn GetDirection
  (bind _staticmesh (Variables|Default|GetStaticMesh))
  (bind _targetref (Variables|Default|GetTargetRef))
  (bind _returnvalue (Transformation|GetWorldLocation _staticmesh))
  (bind _staticmesh_2 (Variables|BP_HookableBox_C|GetStaticMesh _targetref))
  (bind _returnvalue_2 (Transformation|GetWorldLocation _staticmesh_2))
  (return (* (Math|Vector|Normalize (Math|Vector|GetUnitDirection(Vector) _returnvalue _returnvalue_2)) (Variables|Default|GetSpeed)) (Math|Vector|Distance(Vector) _returnvalue _returnvalue_2)))