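; BPC_BuildSystem is an actor component that lets the first-person character preview and place floor pieces.
; While build mode is toggled on, Tick traces from the camera and moves a collision-free preview mesh to the hit point, creating it once via DoOnce.
; Positive RotateObject axis input adds yaw to the preview.
; Placing spawns BP_Build_Floor at the preview transform, then exits build mode, clearing the preview and resetting the DoOnce.
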(event Custom|Preview%20Loop
  (bind _camera (Variables|Default|GetCamera))
  (bind _returnvalue (Transformation|GetWorldTransform _camera))
  (bind (_outhit _returnvalue_2) (Collision|LineTraceByChannel (.location _returnvalue) (+ (.location _returnvalue) (* (Math|Vector|GetForwardVector (.rotation _returnvalue)) 7e+02)) "TraceTypeQuery1" false 0 "None"))
  (if _returnvalue_2
    (Utilities|FlowControl|Sequence
      (:then_0
        (Utilities|FlowControl|DoOnce false
          (:Completed
            (bind _returnvalue_3 (Game|AddComponentbyClass (Variables|Default|GetPlayer%20BP) "/Script/Engine.StaticMeshComponent" false (Variables|Default|GetBuild%20Preview%20transform)))
            (bind _output_get (Variables|Default|SetPreview%20Mesh _returnvalue_3))
            (Components|StaticMesh|SetStaticMesh _output_get "/Game/StarterContent/Architecture/Floor_400x400.Floor_400x400")
            (Rendering|Material|SetMaterial (Variables|Default|GetPreview%20Mesh) 0 "/Game/Blueprint/PreviewMesh.PreviewMesh")
            (Collision|SetCollisionEnabled (Variables|Default|GetPreview%20Mesh) "NoCollision"))))
      (:then_1
        (bind _output_get_2 (Variables|Default|SetBuild%20Preview%20transform (Math|Transform|MakeTransform (.Location (Collision|BreakHitResult _outhit)) (Variables|Default|GetBuildPreviewRotation) "1.000000,1.000000,1.000000")))
        (Transformation|SetWorldTransform (Variables|Default|GetPreview%20Mesh) _output_get_2 false false)))))

(event Custom|ResetBuildMode
  (Utilities|FlowControl|DoOnce false) ; enters at Reset
)

(event Custom|Stop%20Build%20Mode
  (Variables|Default|SetInBuildMode false)
  (Components|StaticMesh|SetStaticMesh (Variables|Default|GetPreview%20Mesh) 0)
  (Variables|Default|SetPreview%20Mesh 0)
  (CallFunction|ResetBuildMode))

(event Input|EnhancedActionEvents|EnhancedInputActionIA_Build
  (params (ActionValue :type Boolean) (ElapsedSeconds :type Float%20%28double-precision%29) (TriggeredSeconds :type Float%20%28double-precision%29) (InputAction :type Input%20Action%20Object%20Reference :default "/Game/FirstPerson/Input/Actions/IA_Build.IA_Build"))
  (:Started
    (if (not (Variables|Default|GetInBuildMode))
      (Variables|Default|SetInBuildMode true)
      (else
        (Variables|Default|SetInBuildMode false)
        (Components|StaticMesh|SetStaticMesh (Variables|Default|GetPreview%20Mesh) 0)
        (Variables|Default|SetPreview%20Mesh 0)
        (CallFunction|ResetBuildMode)))))

(event Input|EnhancedActionEvents|EnhancedInputActionIA_PlaceBuild
  (params (ActionValue :type Boolean) (ElapsedSeconds :type Float%20%28double-precision%29) (TriggeredSeconds :type Float%20%28double-precision%29) (InputAction :type Input%20Action%20Object%20Reference :default "/Game/FirstPerson/Input/Actions/IA_PlaceBuild.IA_PlaceBuild"))
  (:Started
    (if (Variables|Default|GetInBuildMode)
      (Game|SpawnActorfromClass "/Game/Blueprint/BP_Build_Floor.BP_Build_Floor_C" (Variables|Default|GetBuild%20Preview%20transform) "AlwaysSpawn" "MultiplyWithRoot" 0 0)
      (CallFunction|StopBuildMode))))

(event EventBeginPlay
  (bind _asbp_first_person_character (Utilities|Casting|CastToBP_FirstPersonCharacter (Components|GetOwner)))
  (Variables|Default|SetPlayer%20BP _asbp_first_person_character)
  (Variables|Default|SetCamera (Variables|/Game/FirstPerson/Blueprints/BP_FirstPersonCharacter.BP_FirstPersonCharacter_C|GetFirstPersonCamera _asbp_first_person_character)))

(event EventTick
  (params (DeltaSeconds :type Float%20%28single-precision%29))
  (if (Variables|Default|GetInBuildMode)
    (CallFunction|PreviewLoop)))

(event Input|AxisEvents|InputAxisRotateObject
  (params (AxisValue :type Float%20%28single-precision%29))
  (if (> AxisValue 0.0)
    (Variables|Default|SetBuildPreviewRotation (Math|Rotator|MakeRotator 0.0 0.0 (+ (* AxisValue (Variables|Default|GetRotation)) (.Yaw (Math|Rotator|BreakRotator (Variables|Default|GetBuildPreviewRotation))))))))