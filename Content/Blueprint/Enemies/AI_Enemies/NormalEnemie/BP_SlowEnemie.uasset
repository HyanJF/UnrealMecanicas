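; Slow melee enemy character that patrols target points, chases pawns it sees and respawns after dying.
; PawnSensing switches it from looping AIMoveTo patrol to a chase, which ends in an attack montage and delayed sphere trace to apply damage.
; FnDamage plays hit or death montages; death hides it, then restores health and visibility in place after a delay.
; Tick sets walk speed from CanMove, and ACHookable gets the capsule as its object to move.
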(event OnSeePawn(PawnSensing)
  (params (Pawn :type Pawn%20Object%20Reference))
  (Variables|Default|SetIsSeeingPlayer true)
  (CallFunction|ChaseTarget Pawn))

(event Custom|Patrol
  (bind _target_point (Variables|Default|GetTarget%20Point))
  ;[0.15 0.15 0.15 0.5] Patrol Event
  (AI|AIMoveTo self (Transformation|GetActorLocation (Utilities|Array|Get(acopy) _target_point (Variables|Default|GetIndex))) 0 5.0 false
    (:OnSuccess
      (if (>= (Variables|Default|GetIndex) (- (Utilities|Array|Length _target_point) 1))
        (Variables|Default|SetIndex 0)
        (else
          (Math|Integer|IncrementInt (Variables|Default|GetIndex)
            (:%20%20
              _))))
      (CallFunction|Patrol))))

(event Custom|Chase%20Target
  (params (Target%20Actor :type Actor%20Object%20Reference))
  (bind _attackzone (Variables|Default|GetAttackZone))
  (bind _returnvalue (Transformation|GetWorldLocation _attackzone))
  ;[0.15 0.15 0.15 0.5] Attack Player
  (Variables|Default|SetcanAttack? true)
  (if (Variables|Default|GetIsSeeingPlayer)
    (AI|AIMoveTo self "0, 0, 0" Target%20Actor 5.0 false
      (:OnSuccess
        (Variables|Default|SetcanMove? false)
        (if (Variables|Default|GetcanAttack?)
          (Animation|PlayAnimMontage "/Game/Animations/Enemie_Animations/AM_Attack.AM_Attack" 1.0 "None")
          (Utilities|FlowControl|Delay 0.5)
          (Variables|Default|SetcanAttack? false)
          (bind (_outhit _returnvalue_2) (Collision|SphereTraceForObjects _returnvalue _returnvalue 1e+02 (Utilities|Array|MakeArray "ObjectTypeQuery3") false 0 "ForDuration" true "(R=1.000000,G=0.000000,B=0.000000,A=1.000000)" "(R=0.000000,G=1.000000,B=0.000000,A=1.000000)" 1.0))
          (if _returnvalue_2
            (Development|PrintString "Recibiste daño")
            (Game|Damage|ApplyDamage 0 0.0 0 0)
            (else
              (Development|PrintString "No Pego")))))
      (:OnFail
        (Variables|Default|SetcanMove? true)
        (CallFunction|Patrol)))
    (else
      (Variables|Default|SetIsSeeingPlayer false))))

(event Custom|Die
  (Development|PrintString (Utilities|String|Append (Utilities|GetDisplayName self) " was killed") true true "(R=0.000000,G=0.660000,B=1.000000,A=1.000000)" 2.0 "DummyKilled")
  (Rendering|SetActorHiddenInGame true)
  (Utilities|FlowControl|Delay 3.0)
  (Variables|Default|SetCurrentHealth (Variables|Default|GetMaxHealth))
  (Collision|SetCollisionEnabled (Variables|Default|GetCapsuleComponent) "QueryOnly")
  (Rendering|SetActorHiddenInGame false)
  (Variables|Default|SetcanMove? true)
  (Development|PrintString (Utilities|String|Append (Utilities|GetDisplayName self) " has reborned"))
  (Default|CallOnRespawn))

(event EventBeginPlay
  (|CallParentFunction)
  (CallFunction|Patrol)
  (EventDispatchers|BindEventtoOnDead (delegate Custom|Die))
  (Variables|/Game/Blueprint/Components/AC_Hookable.AC_Hookable_C|SetObjectToMove (Variables|Default|GetAC_Hookable) (Variables|Default|GetCapsuleComponent)))

(event Collision|EventActorBeginOverlap
  (params (OtherActor :type Actor%20Object%20Reference))
  (|CallParentFunction OtherActor) ; This node is disabled and will not be called.\nDrag off pins to build functionality.
)

(event EventTick
  (params (DeltaSeconds :type Float%20%28single-precision%29))
  (bind _charactermovement (Variables|Character|GetCharacterMovement))
  (|CallParentFunction DeltaSeconds)
  (if (Variables|Default|GetcanMove?)
    (Variables|/Script/Engine.CharacterMovementComponent|SetMaxWalkSpeed _charactermovement 2e+02)
    (else
      (Variables|/Script/Engine.CharacterMovementComponent|SetMaxWalkSpeed _charactermovement 0.0)))
  (if (not (Variables|Default|GetIsSeeingPlayer))
    (CallFunction|Patrol)))

(event EventFnDamage
  (params (DamageCauser :type Actor%20Object%20Reference) (DamageAmount :type Float%20%28double-precision%29))
  (bind _self self)
  (bind _returnvalue (Utilities|GetDisplayName _self))
  ;[0.15 0.15 0.15 0.5] Damage
  (Development|PrintString (Utilities|String|Append (Utilities|GetDisplayName DamageCauser) " dealed " (Utilities|String|ToString(Float) DamageAmount) " damage to " _returnvalue " new HP " (Utilities|String|ToString(Float) (Variables|Default|GetCurrentHealth))) true true "(R=0.000000,G=0.660000,B=1.000000,A=1.000000)" 2.0 (Utilities|String|StringToName _returnvalue))
  (bind _output_get (Variables|Default|SetCurrentHealth (- (Variables|Default|GetCurrentHealth) DamageAmount)))
  (if (<= _output_get 0.0)
    (Collision|SetCollisionEnabled (Variables|Default|GetCapsuleComponent) "NoCollision")
    (Variables|Default|SetcanMove? false)
    (bind _returnvalue_2 (Animation|PlayAnimMontage "/Game/Animations/Enemie_Animations/AM_Death.AM_Death" 1.0 "None"))
    (Utilities|FlowControl|Delay _returnvalue_2)
    (Default|CallOnDead)
    (else
      (Animation|PlayAnimMontage "/Game/Animations/Enemie_Animations/AM_Hit.AM_Hit" 1.0 "None"))))

(fn ConstructionScript
  (|CallParentFunction))