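; BP_EnemyDummie is a dummy enemy that takes damage, dies and respawns with full health after a short delay.
; Its damage event logs the hit, subtracts health and calls OnDead at zero, with the logged "new HP" read before subtraction.
; The bound Die handler hides the actor and disables collision, then restores both and calls OnRespawn.
; BeginPlay also sets BodyCollition as the object its ACHookable component moves.
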(event Custom|Die
  (Development|PrintString (Utilities|String|Append (Utilities|GetDisplayName self) " was killed") true true "(R=0.000000,G=0.660000,B=1.000000,A=1.000000)" 2.0 "DummyKilled")
  (Collision|SetActorEnableCollision false)
  (Rendering|SetActorHiddenInGame true)
  (Utilities|FlowControl|Delay 3.0)
  (Variables|Default|SetCurrentHealth (Variables|Default|GetMaxHealth))
  (Collision|SetActorEnableCollision true)
  (Rendering|SetActorHiddenInGame false)
  (Development|PrintString (Utilities|String|Append (Utilities|GetDisplayName self) " has reborned"))
  (Default|CallOnRespawn))

(event EventBeginPlay
  (|CallParentFunction)
  (EventDispatchers|BindEventtoOnDead (delegate Custom|Die))
  (Variables|/Game/Blueprint/Components/AC_Hookable.AC_Hookable_C|SetObjectToMove (Variables|Default|GetAC_Hookable) (Variables|Default|GetBodyCollition)))

(event EventFnDamage
  (params (DamageCauser :type Actor%20Object%20Reference) (DamageAmount :type Float%20%28double-precision%29))
  (bind _self self)
  (bind _returnvalue (Utilities|GetDisplayName _self))
  (Development|PrintString (Utilities|String|Append (Utilities|GetDisplayName DamageCauser) " dealed " (Utilities|String|ToString(Float) DamageAmount) " damage to " _returnvalue " new HP " (Utilities|String|ToString(Float) (Variables|Default|GetCurrentHealth))) true true "(R=0.000000,G=0.660000,B=1.000000,A=1.000000)" 2.0 (Utilities|String|StringToName _returnvalue))
  (bind _output_get (Variables|Default|SetCurrentHealth (- (Variables|Default|GetCurrentHealth) DamageAmount)))
  (if (<= _output_get 0.0)
    (Default|CallOnDead)))

(fn ConstructionScript
  (|CallParentFunction))