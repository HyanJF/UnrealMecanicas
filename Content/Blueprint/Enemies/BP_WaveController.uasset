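; BP_WaveController runs endless, escalating enemy waves and keeps the wave HUD up to date.
; On BeginPlay it creates WB_WaveUI and starts a wave, passing per-type counts (fast, normal, slow) and itself to each spawner.
; EnemyAlive and enemyDied events maintain the living count and update the widget.
; When that count hits zero, it waits, raises each spawn count by one and starts the next wave.
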(event Custom|StartWave
  (Variables|/Game/Blueprint/Widgets/WB_WaveUI.WB_WaveUI_C|SetRoundNumber (Variables|Default|GetWaveUi) (Variables|Default|GetcurrentWave))
  (Variables|Default|SetIsWaveInProgress true)
  (for _array_element (Variables|Default|GetSpawners)
    (Default|StartSpawnLoop _array_element (Variables|Default|GetFastToSpawn) (Variables|Default|GetNormalToSpawn) (Variables|Default|GetSlowToSpawn) self)))

(event Custom|EnemyAlive
  (bind _output_get (Variables|Default|SetEnemiesAlive (+ (Variables|Default|GetEnemiesAlive) 1)))
  (Variables|/Game/Blueprint/Widgets/WB_WaveUI.WB_WaveUI_C|SetEnemiesRemaining (Variables|Default|GetWaveUi) _output_get))

(event Custom|enemyDied
  (bind _output_get (Variables|Default|SetEnemiesAlive (- (Variables|Default|GetEnemiesAlive) 1)))
  (Variables|/Game/Blueprint/Widgets/WB_WaveUI.WB_WaveUI_C|SetEnemiesRemaining (Variables|Default|GetWaveUi) _output_get)
  (if (== (Variables|Default|GetEnemiesAlive) 0)
    (Utilities|FlowControl|Delay 15.0)
    (Variables|Default|SetFastToSpawn (+ (Variables|Default|GetFastToSpawn) 1))
    (Variables|Default|SetNormalToSpawn (+ (Variables|Default|GetNormalToSpawn) 1))
    (Variables|Default|SetSlowToSpawn (+ (Variables|Default|GetSlowToSpawn) 1))
    (Variables|Default|SetcurrentWave (+ (Variables|Default|GetcurrentWave) 1))
    (CallFunction|StartWave)))

(event EventBeginPlay
  (bind _returnvalue (UserInterface|CreateWidget "/Game/Blueprint/Widgets/WB_WaveUI.WB_WaveUI_C" 0 (Variables|Default|GetcurrentWave) (Variables|Default|GetEnemiesAlive)))
  (Variables|Default|SetWaveUi _returnvalue)
  (UserInterface|Viewport|AddtoViewport (Variables|Default|GetWaveUi) 0)
  (CallFunction|StartWave))

(event Collision|EventActorBeginOverlap
  (params (OtherActor :type Actor%20Object%20Reference)))

(event EventTick
  (params (DeltaSeconds :type Float%20%28single-precision%29)))

(fn ConstructionScript)