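; BP_FixedMoveEnemy is an enemy that patrols back and forth along a straight path between Start and End offsets from its root's location.
; A half-speed timeline lerps the body collision between the offsets, and each finish calls Move, which flips IsInReverse to alternate direction.
; Death stops the timeline and pre-flips the flag, so the Move call on respawn resumes in the interrupted direction.
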(event Custom|Play
  (bind _movetime (Timeline|MoveTimeLine Play)
    (:Update
      (Transformation|SetWorldTransform (Variables|Default|GetBodyCollition) (Math|Transform|MakeTransform (+ (Math|Vector|Lerp(Vector) (Variables|Default|GetStart) (Variables|Default|GetEnd) _movetime) (.location (Transformation|GetWorldTransform (Variables|Default|GetDefaultSceneRoot)))) "0, 0, 0" "1.000000,1.000000,1.000000") false false))
    (:Finished
      (CallFunction|Move))))

(event Custom|Reverse
  (bind _movetime (Timeline|MoveTimeLine Reverse)
    (:Update
      (Transformation|SetWorldTransform (Variables|Default|GetBodyCollition) (Math|Transform|MakeTransform (+ (Math|Vector|Lerp(Vector) (Variables|Default|GetStart) (Variables|Default|GetEnd) _movetime) (.location (Transformation|GetWorldTransform (Variables|Default|GetDefaultSceneRoot)))) "0, 0, 0" "1.000000,1.000000,1.000000") false false))
    (:Finished
      (CallFunction|Move))))

(event Custom|StopMoving
  (Variables|Default|SetIsInReverse (not (Variables|Default|GetIsInReverse)))
  (bind _movetime (Timeline|MoveTimeLine Stop)
    (:Update
      (Transformation|SetWorldTransform (Variables|Default|GetBodyCollition) (Math|Transform|MakeTransform (+ (Math|Vector|Lerp(Vector) (Variables|Default|GetStart) (Variables|Default|GetEnd) _movetime) (.location (Transformation|GetWorldTransform (Variables|Default|GetDefaultSceneRoot)))) "0, 0, 0" "1.000000,1.000000,1.000000") false false))
    (:Finished
      (CallFunction|Move))))

(event Custom|Respawn
  (CallFunction|Move))

(event Custom|Move
  ;[0.15 0.15 0.15 0.5] Move
  (bind _output_get (Variables|Default|SetIsInReverse (not (Variables|Default|GetIsInReverse))))
  (if _output_get
    (CallFunction|Reverse)
    (else
      (CallFunction|Play))))

(event EventBeginPlay
  (|CallParentFunction)
  (Components|Timeline|SetPlayRate (Variables|Default|GetMoveTimeLine) 0.5)
  (EventDispatchers|BindEventtoOnRespawn (delegate Custom|Respawn))
  (EventDispatchers|BindEventtoOnDead (delegate Custom|StopMoving))
  (bind _movetime (Timeline|MoveTimeLine Play)
    (:Update
      (Transformation|SetWorldTransform (Variables|Default|GetBodyCollition) (Math|Transform|MakeTransform (+ (Math|Vector|Lerp(Vector) (Variables|Default|GetStart) (Variables|Default|GetEnd) _movetime) (.location (Transformation|GetWorldTransform (Variables|Default|GetDefaultSceneRoot)))) "0, 0, 0" "1.000000,1.000000,1.000000") false false))
    (:Finished
      (CallFunction|Move))))

(fn ConstructionScript
  (|CallParentFunction))